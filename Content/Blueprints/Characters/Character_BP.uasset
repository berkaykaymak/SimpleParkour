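; Player character Blueprint with walk, look, jump and crouch input, plus a bunny-hop style speed boost.
; Each jump made while moving raises max walk speed in steps up to a cap.
; The forward axis event tracks movement from velocity and jumping from vertical velocity with a retriggerable delay, resetting speed when the character stops or stays out of a jump.
; That event also prints speed and movement state for debugging.
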(event `self.OnJumped`
  (bind _charactermovement (`self.CharacterMovement`))
  (bind _returnvalue (`MovementComponent.GetMaxSpeed` _charactermovement))
  ;[1 1 1] Acceleration on Event Jump
  (if (`self.IsMoving?`)
    (if (< _returnvalue 1200.0)
      (set `CharacterMovementComponent.MaxWalkSpeed` (+ _returnvalue 100.0) _charactermovement))))

(event `InputAxis|ForwardBacwardMovement`
  (params (AxisValue :type "Float (single-precision)"))
  (bind (_returnvalue_x _returnvalue_y _returnvalue_z) (`KismetMathLibrary.BreakVector` (`self.GetVelocity`)))
  (bind (_returnvalue_roll _returnvalue_pitch _returnvalue_yaw) (`KismetMathLibrary.BreakRotator` (`self.GetControlRotation`)))
  (bind _returnvalue (`KismetMathLibrary.VSize` (`KismetMathLibrary.MakeVector` _returnvalue_x _returnvalue_y _returnvalue_z)))
  ;[1 1 1] Movement
  (`self.AddMovementInput` (`KismetMathLibrary.GetForwardVector` (`KismetMathLibrary.MakeRotator` 0.0 0.0 _returnvalue_yaw)) AxisValue)
  (`|ExecutionSequence`
    (:`then_0`
      ;[1 1 1] Acceleration on Event Jump
      (`KismetSystemLibrary.PrintString` (`KismetStringLibrary.Conv_IntToString` (`KismetMathLibrary.FFloor` _returnvalue)) true true (struct :`G` 0.66 :`B` 1.0 :`A` 1.0) 0.0)
      (if (!= _returnvalue 0.0)
        (set `self.IsMoving?` true)
        (`KismetSystemLibrary.PrintString` "Moving" true true (struct :`G` 0.66 :`B` 1.0 :`A` 1.0) 0.0)
        (else
          (set `self.IsMoving?` false)
          (`KismetSystemLibrary.PrintString` "Not Moving" true true (struct :`G` 0.66 :`B` 1.0 :`A` 1.0) 0.0)
          (set `CharacterMovementComponent.MaxWalkSpeed` 600.0 (`self.CharacterMovement`)))))
    (:`then_1`
      (if (!= _returnvalue_z 0.0)
        (set `self.IsJumping?` true)
        (`KismetSystemLibrary.RetriggerableDelay` 0.7)
        (set `self.IsJumping?` false)))
    (:`then_2`
      (if (not (`self.IsJumping?`))
        (set `CharacterMovementComponent.MaxWalkSpeed` 600.0 (`self.CharacterMovement`))))))

(event `InputAction|JumpAction`
  (params (Key :type "Key Structure"))
  ;[1 1 1] MouseMovements
  (:`Pressed`
    (`self.Jump`))
  (:`Released`
    (`self.StopJumping`)))

(event `InputAction|CrouchAction`
  (params (Key :type "Key Structure"))
  ;[1 1 1] MouseMovements
  (:`Pressed`
    (`self.Crouch`))
  (:`Released`
    (`self.UnCrouch`)))

(event `InputAxis|RightLeftMovement`
  (params (AxisValue :type "Float (single-precision)"))
  (bind (_returnvalue_roll _returnvalue_pitch _returnvalue_yaw) (`KismetMathLibrary.BreakRotator` (`self.GetControlRotation`)))
  ;[1 1 1] Movement
  (`self.AddMovementInput` (`KismetMathLibrary.GetRightVector` (`KismetMathLibrary.MakeRotator` 0.0 0.0 _returnvalue_yaw)) AxisValue))

(event `InputAxis|UpDownLooking`
  (params (AxisValue :type "Float (single-precision)"))
  (`self.AddControllerPitchInput` AxisValue))

(event `InputAxis|RightLeftLooking`
  (params (AxisValue :type "Float (single-precision)"))
  (`self.AddControllerYawInput` AxisValue))

(fn `UserConstructionScript`)